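; Player controller for the Starfighter minigame that handles the pre-spawn team selection phase.
; On BeginPlay the authority possesses the first StartViewPawn in the level, then a team selection widget is shown with UI-only input and a visible cursor.
; A TeamSelected event forwards the chosen team and this controller to BP_Starfighter_Gamemode to request a spawn.
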(event Custom|TeamSelected
  (params (team :type TeamEnum%20Enum :default "NewEnumerator0"))
  (Default|RequestSpawn (.AsBP%20Starfighter%20Gamemode (Utilities|Casting|CastToBP_Starfighter_Gamemode (Game|GetGameMode))) team self))

(event EventBeginPlay
  (bind _self self)
  ;[1 1 1] Add Widget Menu To Viewport
  (Utilities|FlowControl|Sequence
    (:then_0
      (Networking|SwitchHasAuthority
        (:Authority
          (bind _outactors (Actor|GetAllActorsOfClass "/Game/Minigames/Starfighter/StartViewPawn.StartViewPawn_C"))
          (Pawn|Possess (Utilities|Array|Get(acopy) _outactors)))))
    (:then_1
      (bind _returnvalue (UserInterface|CreateWidget "/Game/Minigames/Starfighter/WBP_StarfighterTeamSelection.WBP_StarfighterTeamSelection_C"))
      (Input|SetInputModeUIOnly _self _returnvalue "DoNotLock")
      (Variables|/Script/Engine.PlayerController|SetbShowMouseCursor _self true)
      (UserInterface|Viewport|AddtoViewport _returnvalue 0))))

(event EventTick
  (params (DeltaSeconds :type Float%20%28single-precision%29)))

(fn ConstructionScript)