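; Game mode for the Starfighter minigame that spawns players into team-specific starfighters.
; RequestSpawn takes a team and controller, then picks a random PlayerStart tagged RedTeam for Team A or BlueTeam for Team B.
; It spawns that team's ship there, adjusting for collisions, has the controller possess it, and adds the ship to the game state's Players list.
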(event Custom|RequestSpawn
  (params (Team :type TeamEnum%20Enum :default "NewEnumerator0") (Controller :type Controller%20Object%20Reference))
  (bind _returnvalue (Game|GetGameState))
  (bind _asbp_starfighter_game_state (Utilities|Casting|CastToBP_Starfighter_GameState _returnvalue))
  (bind _players (Variables|/Game/Minigames/Starfighter/BP_Starfighter_GameState.BP_Starfighter_GameState_C|GetPlayers _asbp_starfighter_game_state))
  ;[1 1 1] Spawn Player on a Certain Team
  (switch Utilities|FlowControl|Switch|SwitchonTeamEnum Team
    (:NewEnumerator0
      (bind _outactors (Actor|GetAllActorsOfClasswithTag "/Script/Engine.PlayerStart" "RedTeam"))
      (bind _returnvalue_2 (Game|SpawnActorfromClass "/Game/Minigames/Starfighter/Starfighter_Models/Starfighter_TeamA_BP.Starfighter_TeamA_BP_C" (Transformation|GetActorTransform (Utilities|Array|Get(acopy) _outactors (Math|Random|RandomInteger (Utilities|Array|Length _outactors)))) "AdjustIfPossibleButAlwaysSpawn" 0 0))
      (Pawn|Possess Controller _returnvalue_2)
      (Utilities|Array|AddUnique _players _returnvalue_2))
    (:NewEnumerator1
      (bind _outactors_2 (Actor|GetAllActorsOfClasswithTag "/Script/Engine.PlayerStart" "BlueTeam"))
      (bind _returnvalue_3 (Game|SpawnActorfromClass "/Game/Minigames/Starfighter/Starfighter_Models/Starfighter_TeamB_BP.Starfighter_TeamB_BP_C" (Transformation|GetActorTransform (Utilities|Array|Get(acopy) _outactors_2 (Math|Random|RandomInteger (Utilities|Array|Length _outactors_2)))) "AdjustIfPossibleButAlwaysSpawn" 0 0))
      (Pawn|Possess Controller _returnvalue_3)
      (Utilities|Array|AddUnique _players _returnvalue_3))))

(event EventBeginPlay)

(event EventTick
  (params (DeltaSeconds :type Float%20%28single-precision%29)))

(fn ConstructionScript)